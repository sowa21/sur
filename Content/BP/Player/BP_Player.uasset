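; Player character Blueprint that turns input into movement, sprinting, jumping, mouse look and camera switching.
; MoveForward sets max walk speed through a Sequence of overrides, where backpedal and strafe take precedence over sprint.
; Sprint engages only if the axis value is fully forward when pressed, and MoveRight flags strafing.
; A FlipFlop toggles between the main and extra cameras, and jumping sets a flag never cleared here.
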(event Input|ActionEvents|InputActionchangecamera
  (params (Key :type Key%20Structure :default "None"))
  ;[1 1 1] камера 1вид
  (:Pressed
    (Utilities|FlowControl|FlipFlop
      (:A
        (Components|Activation|Deactivate (Variables|Default|GetCamera))
        (Components|Activation|Activate (Variables|Default|GetExtraCamera) false))
      (:B
        (Components|Activation|Deactivate (Variables|Default|GetExtraCamera))
        (Components|Activation|Activate (Variables|Default|GetCamera) false)))))

(event Input|ActionEvents|InputActionSprintg
  (params (Key :type Key%20Structure :default "None"))
  ;[1 1 1] бег
  (:Pressed
    (if (== (stale Input|AxisEvents|InputAxisMoveForward AxisValue) 1.0)
      (Variables|Default|Setissprinting? true)
      (else
        (Variables|Default|Setissprinting? false))))
  (:Released
    (Variables|Default|Setissprinting? false)))

(event Input|ActionEvents|InputActionJump
  (params (Key :type Key%20Structure :default "None"))
  ;[1 1 1] прыжок
  (:Pressed
    (Character|Jump)
    (Variables|Default|Setisjumping true)))

(event Input|AxisEvents|InputAxisMoveForward
  (params (AxisValue :type Float%20%28single-precision%29))
  (bind _charactermovement (Variables|Character|GetCharacterMovement))
  ;[1 1 1] движение
  (Pawn|Input|AddMovementInput (Math|Vector|GetForwardVector (Variables|Collision|GetCapsuleComponent)) AxisValue false)
  (Utilities|FlowControl|Sequence
    (:then_0
      ;[1 1 1] ходьба
      (Variables|/Script/Engine.CharacterMovementComponent|SetMaxWalkSpeed _charactermovement 3e+02))
    (:then_1
      ;[1 1 1] ходьба назад
      (if (== AxisValue -1.0)
        (Variables|/Script/Engine.CharacterMovementComponent|SetMaxWalkSpeed _charactermovement 1.5e+02)))
    (:then_2
      ;[1 1 1] бег(скорость)
      (if (Variables|Default|Getissprinting?)
        (Variables|/Script/Engine.CharacterMovementComponent|SetMaxWalkSpeed _charactermovement 6e+02)))
    (:then_3
      ;[1 1 1] скорость стрейфа
      (if (Variables|Default|GetisWalkRight)
        (Variables|/Script/Engine.CharacterMovementComponent|SetMaxWalkSpeed (Variables|Character|GetCharacterMovement) 3e+02)))
    (:then_4
      ;[1 1 1] Comment
      (if (== AxisValue -1.0)
        (Variables|/Script/Engine.CharacterMovementComponent|SetMaxWalkSpeed (Variables|Character|GetCharacterMovement) 1.5e+02)))))

(event Input|AxisEvents|InputAxisMoveRight
  (params (AxisValue :type Float%20%28single-precision%29))
  ;[1 1 1] движение
  (Pawn|Input|AddMovementInput (Math|Vector|GetRightVector (Variables|Collision|GetCapsuleComponent)) AxisValue false)
  ;[1 1 1] влево/вправо
  (Variables|Default|SetisWalkRight (or (== AxisValue -1.0) (== AxisValue 1.0))))

(event Input|AxisEvents|InputAxislookUp
  (params (AxisValue :type Float%20%28single-precision%29))
  ;[1 1 1] мышь
  (Pawn|Input|AddControllerPitchInput AxisValue))

(event Input|AxisEvents|InputAxislookright
  (params (AxisValue :type Float%20%28single-precision%29))
  ;[1 1 1] мышь
  (Pawn|Input|AddControllerYawInput AxisValue))

(fn ConstructionScript)